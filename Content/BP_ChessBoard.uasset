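; Chess board actor that spawns two chequer pawns on opposite grid nodes and runs an AI movement test between them.
; On BeginPlay, two delayed sequence branches each spawn a pawn and set its movement component's current node.
; Completion flags join the branches, then AIMovementTask runs with the first pawn's AI controller and the second pawn as the chequer, printing success or failure.
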(event `self.ReceiveBeginPlay`
  (bind _returnvalue (`self.GetNode` (make `GridVector` 0)))
  (bind _returnvalue_2 (`self.GetNode` (make `GridVector` 5 5)))
  (`KismetSystemLibrary.Delay` 0.2)
  (`|ExecutionSequence`
    (:`then_0`
      (bind _returnvalue_3 (`|SpawnActorFromClass` "/Game/BP_ChequerPawn.BP_ChequerPawn_C" (`KismetMathLibrary.MakeTransform` (`BoardNode.Location` _returnvalue)) "AlwaysSpawn" "OverrideRootScale" null null))
      (`KismetSystemLibrary.Delay` 0.2)
      (`ChequerMovementComponent.SetCurrentNode` (`/Game/BP_ChequerPawn.ChequerMovement` _returnvalue_3) _returnvalue)
      (bind _output_get (set `self.First Complete` true)))
    (:`then_1`
      (bind _returnvalue_4 (`|SpawnActorFromClass` "/Game/BP_ChequerPawn.BP_ChequerPawn_C" (`KismetMathLibrary.MakeTransform` (`BoardNode.Location` _returnvalue_2)) "AlwaysSpawn" "OverrideRootScale" null null))
      (`KismetSystemLibrary.Delay` 0.2)
      (`ChequerMovementComponent.SetCurrentNode` (`/Game/BP_ChequerPawn.ChequerMovement` _returnvalue_4) _returnvalue_2)
      (bind _output_get_2 (set `self.Second Complete` true))))
  (if (and _output_get _output_get_2)
    (`AITask_Movement.CreateAIMovementTask` (`AIBlueprintHelperLibrary.GetAIController` _returnvalue_3) null _returnvalue_4
      (:`OnTaskSucceeded`
        (`KismetSystemLibrary.PrintString` "1"))
      (:`OnTaskFailed`
        (`KismetSystemLibrary.PrintString` "0")))))

(fn `UserConstructionScript`)