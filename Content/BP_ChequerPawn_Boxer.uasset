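; Boxer chess-piece pawn, a child Blueprint that customizes how the piece deals damage.
; MakeDamage raises Health by a fifth of its current value when Mana is at or above ManaMax, with no clamp or Mana reset here.
; It then applies AttackPower as damage to CurrentTarget in every case.
; The construction script only calls the parent, and the event graph holds only disabled placeholder events.
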(fn `MakeDamage`
  (bind _health (`self.Health`))
  (set `self.Health` (`KismetMathLibrary.SelectFloat` (+ (/ (`self.Health`) 5.0) _health) _health (>= (`self.Mana`) (`self.ManaMax`))))
  (`GameplayStatics.ApplyDamage` (`self.CurrentTarget`) (`KismetMathLibrary.Conv_IntToDouble` (`self.AttackPower`))))

(fn `UserConstructionScript`
  (`parent.UserConstructionScript`))